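; BP_Camera is the RTS camera pawn in the PlayerPawn folder, which the player moves and rotates through axis inputs.
; The forward and right axes offset the actor along its own vectors by a fixed step, without sweep or delta-time scaling.
; Look axes add controller pitch and yaw only while the PC_RTS controller, cached on BeginPlay, is not selecting.
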(event `self.ReceiveBeginPlay`
  (bind _aspc_rts (cast `/Game/PlayerPawn/PC_RTS` (`GameplayStatics.GetPlayerController` 0)))
  (set `self.PlayerController` _aspc_rts))

(event `InputAxis|fwd`
  (params (AxisValue :type "Float (single-precision)"))
  (`self.K2_SetActorLocation` (+ (* (`self.GetActorForwardVector`) (* AxisValue 10.0)) (`self.K2_GetActorLocation`))))

(event `InputAxis|rght`
  (params (AxisValue :type "Float (single-precision)"))
  (`self.K2_SetActorLocation` (+ (* (`self.GetActorRightVector`) (* AxisValue 10.0)) (`self.K2_GetActorLocation`))))

(event `InputAxis|LookUp`
  (params (AxisValue :type "Float (single-precision)"))
  (if (not (`/Game/PlayerPawn/PC_RTS.Selecting` (`self.PlayerController`)))
    (`self.AddControllerPitchInput` AxisValue)))

(event `InputAxis|LookLeft`
  (params (AxisValue :type "Float (single-precision)"))
  (if (not (`/Game/PlayerPawn/PC_RTS.Selecting` (`self.PlayerController`)))
    (`self.AddControllerYawInput` AxisValue)))

(fn `UserConstructionScript`)