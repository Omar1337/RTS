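; RTS player controller that drag-selects CH_Unit_PC units and issues move orders under the cursor.
; On select press, AmCommanding chooses between spawning a BP_MoveOrder at a navigable point for all selected units and spawning a BP_Select sphere.
; A looping timer, gated to the drag, scales the sphere by cursor distance.
; Release stores overlapping units in Command and shows their markers; Deselect clears them.
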(event `self.ReceiveBeginPlay`
  (`KismetSystemLibrary.K2_SetTimerDelegate` (delegate `TickAlt`) 0.05 true))

(event `TickAlt`
  (`/Engine/EditorBlueprintResources/StandardMacros.Gate` true :!label _label
    (:`Exit`
      (`/Game/AI_Systems/Selection/BP_Select.ScaleSphere` (`self.Selection`) (/ (`KismetMathLibrary.VSize` (- (`self.P1`) (`.ImpactPoint` (`GameplayStatics.BreakHitResult` (`self.GetHitResultUnderCursorByChannel` "TraceTypeQuery1"))))) 50.0)))))

(event `InputAction|Quit`
  (params (Key :type "Key Structure"))
  (:`Pressed`
    (`KismetSystemLibrary.QuitGame` null "Quit")))

(event `InputAction|select`
  (params (Key :type "Key Structure"))
  (bind _p1 (`self.P1`))
  (:`Pressed`
    (set `self.P1` (`.ImpactPoint` (`GameplayStatics.BreakHitResult` (`self.GetHitResultUnderCursorByChannel` "TraceTypeQuery1"))))
    (if (`self.AmCommanding`)
      (if (`.ReturnValue` (`NavigationSystemV1.K2_ProjectPointToNavigation` _p1))
        (bind _returnvalue (`|SpawnActorFromClass` "/Game/AI_Systems/Orders/BP_MoveOrder.BP_MoveOrder_C" (`KismetMathLibrary.Conv_VectorToTransform` _p1) "Undefined" "OverrideRootScale" null null))
        (`self.AssignOrder` _returnvalue))
      (else
        (set `self.Selecting` true)
        (bind _returnvalue_2 (`|SpawnActorFromClass` "/Game/AI_Systems/Selection/BP_Select.BP_Select_C" (`KismetMathLibrary.Conv_VectorToTransform` (`self.P1`)) "Undefined" "OverrideRootScale" null null))
        (set `self.Selection` _returnvalue_2)
        (goto _label :!via `Open`))))
  (:`Released`
    (if (`self.Selecting`)
      (set `self.Selecting` false)
      (set `self.Command` (`PrimitiveComponent.GetOverlappingActors` (`/Game/AI_Systems/Selection/BP_Select.Sphere` (`self.Selection`)) "/Game/AI_Systems/Actors/CH_Unit_PC.CH_Unit_PC_C"))
      (`self.ShowSelection` true)
      (`|ExecutionSequence`
        (:`then_0`
          (goto _label :!via `Close`))
        (:`then_1`
          (`self.K2_DestroyActor` (`self.Selection`)))))))

(event `InputAction|Deselect`
  (params (Key :type "Key Structure"))
  (:`Pressed`
    (`self.ShowSelection` false)
    (`KismetArrayLibrary.Array_Clear` (`self.Command`))))

(fn `AssignOrder`
  (params (Order :type "/Game/AI_Systems/Orders/BP_MoveOrder Object Reference"))
  (for _array_element (`self.Command`)
    (bind _asch_unit_pc (cast `/Game/AI_Systems/Actors/CH_Unit_PC` _array_element))
    (`/Game/AI_Systems/Actors/CH_Unit_PC.SetOrder` _asch_unit_pc Order)))

(fn `ShowSelection`
  (params (Show :type Boolean))
  (for _array_element (`self.Command`)
    (bind _asch_unit_pc (cast `/Game/AI_Systems/Actors/CH_Unit_PC` _array_element))
    (`SceneComponent.SetHiddenInGame` (`/Game/AI_Systems/Actors/CH_Unit_PC. Selected` _asch_unit_pc) (not Show) false)))

(fn `UserConstructionScript`)